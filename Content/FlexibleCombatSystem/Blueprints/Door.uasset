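; Door Blueprint that opens for BP_PlayerCharacter only when its referenced Enemy is dead.
; Entering the trigger box restores half of the player's max Health and Stamina, capped at maximum, on every qualifying overlap.
; It then snaps the mesh upward with a local offset, and leaving the box lowers it again.
; A separate ChangeMaterial event swaps the mesh's material.
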(event `Change Material`
  (`PrimitiveComponent.SetMaterial` (`self.StaticMesh`) 0 "/DatasmithContent/Materials/AliasReference.AliasReference"))

(event `self.Box.OnComponentBeginOverlap`
  (params (OverlappedComponent :type "PrimitiveComponent Object Reference") (OtherActor :type "Actor Object Reference") (OtherComp :type "PrimitiveComponent Object Reference") (OtherBodyIndex :type Integer) (bFromSweep :type Boolean) (SweepResult :type "HitResult Structure (by ref)"))
  (bind _maxhealth (`/Game/FlexibleCombatSystem/Blueprints/BP_PlayerCharacter.MaxHealth` (`self.As BP Player Character`)))
  (bind _maxstamina (`/Game/FlexibleCombatSystem/Blueprints/BP_PlayerCharacter.MaxStamina` (`self.As BP Player Character`)))
  (bind _returnvalue (+ (`/Game/FlexibleCombatSystem/Blueprints/BP_PlayerCharacter.Stamina` (`self.As BP Player Character`)) (/ _maxstamina 2)))
  (bind _asbp_player_character (cast `/Game/FlexibleCombatSystem/Blueprints/BP_PlayerCharacter` OtherActor))
  (bind _output_get (set `self.As BP Player Character` _asbp_player_character))
  (if (`/Game/FlexibleCombatSystem/Blueprints/AI/BP_EnemyAI.Dead?` (`self.Enemy`))
    (bind _returnvalue_2 (+ (`/Game/FlexibleCombatSystem/Blueprints/BP_PlayerCharacter.Health` _output_get) (/ _maxhealth 2)))
    (if (> _returnvalue_2 _maxhealth)
      (set `/Game/FlexibleCombatSystem/Blueprints/BP_PlayerCharacter.Health` _maxhealth (`self.As BP Player Character`))
      (else
        (set `/Game/FlexibleCombatSystem/Blueprints/BP_PlayerCharacter.Health` _returnvalue_2 (`self.As BP Player Character`))))
    (if true
      (if (> _returnvalue _maxstamina)
        (set `/Game/FlexibleCombatSystem/Blueprints/BP_PlayerCharacter.Stamina` _maxstamina (`self.As BP Player Character`))
        (else
          (set `/Game/FlexibleCombatSystem/Blueprints/BP_PlayerCharacter.Stamina` _returnvalue (`self.As BP Player Character`))))
      (if true
        (`SceneComponent.K2_AddLocalOffset` (`self.StaticMesh`) (0.0 0.0 400.0) false false)))))

(event `self.Box.OnComponentEndOverlap`
  (params (OverlappedComponent :type "PrimitiveComponent Object Reference") (OtherActor :type "Actor Object Reference") (OtherComp :type "PrimitiveComponent Object Reference") (OtherBodyIndex :type Integer))
  (cast `/Game/FlexibleCombatSystem/Blueprints/BP_PlayerCharacter` OtherActor)
  (if (`/Game/FlexibleCombatSystem/Blueprints/AI/BP_EnemyAI.Dead?` (`self.Enemy`))
    (`SceneComponent.K2_AddLocalOffset` (`self.StaticMesh`) (0.0 0.0 -400.0) false false)))

(fn `UserConstructionScript`)