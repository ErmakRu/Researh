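; BP_AttackDefend is an actor that tracks the player's attack and block state and can be removed by the player once both register.
; BeginPlay caches the player character; Tick swaps the mesh material when AttackLMB is at least 1 and BlockSpeedTime is non-empty.
; The material doubles as the completion flag: a player overlapping the box destroys the actor only after the swap.
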(event `self.ReceiveBeginPlay`
  (bind _asbp_player_character (cast `/Game/FlexibleCombatSystem/Blueprints/BP_PlayerCharacter` (`GameplayStatics.GetPlayerCharacter` 0)))
  (set `self.As BP Player Character` _asbp_player_character))

(event `self.ReceiveTick`
  (params (DeltaSeconds :type "Float (single-precision)"))
  (bind _as_bp_player_character (`self.As BP Player Character`))
  (if (and (>= (`/Game/FlexibleCombatSystem/Blueprints/BP_PlayerCharacter.AttackLMB ` _as_bp_player_character) 1) (!= (`BlueprintSetLibrary.Set_Length` (`/Game/FlexibleCombatSystem/Blueprints/BP_PlayerCharacter.BlockSpeedTime` _as_bp_player_character)) 0))
    (`PrimitiveComponent.SetMaterial` (`self.StaticMesh`) 0 "/DatasmithContent/Materials/AliasReference.AliasReference")))

(event `self.Box.OnComponentBeginOverlap`
  (params (OverlappedComponent :type "PrimitiveComponent Object Reference") (OtherActor :type "Actor Object Reference") (OtherComp :type "PrimitiveComponent Object Reference") (OtherBodyIndex :type Integer) (bFromSweep :type Boolean) (SweepResult :type "HitResult Structure (by ref)"))
  (if (== (`PrimitiveComponent.GetMaterial` (`self.StaticMesh`) 0) "/DatasmithContent/Materials/AliasReference.AliasReference")
    (cast `/Game/FlexibleCombatSystem/Blueprints/BP_PlayerCharacter` OtherActor)
    (`self.K2_DestroyActor`)))

(fn `UserConstructionScript`)