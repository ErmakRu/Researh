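; Level-exit sphere trigger that, once the assigned enemy is dead, records player combat telemetry for research and opens the next level.
; On overlap it averages block timings and saves them with attack, block, damage and movement counters as one text file per stat.
; The last level instead sums three arenas plus dead-player files, splitting Arena2 attacks and blocks into inverse counters.
; It writes totals to a hardcoded C: folder and shows WB_FinalScreen.
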(event `self.Sphere.OnComponentBeginOverlap`
  (params (OverlappedComponent :type "PrimitiveComponent Object Reference") (OtherActor :type "Actor Object Reference") (OtherComp :type "PrimitiveComponent Object Reference") (OtherBodyIndex :type Integer) (bFromSweep :type Boolean) (SweepResult :type "HitResult Structure (by ref)"))
  (bind _blockspeedtime (`/Game/FlexibleCombatSystem/Blueprints/BP_PlayerCharacter.BlockSpeedTime` (`self.BP Player Character`)))
  (bind _deltablock (`/Game/FlexibleCombatSystem/Blueprints/BP_PlayerCharacter.DeltaBlock` (`self.BP Player Character`)))
  (bind _asbp_player_character (cast `/Game/FlexibleCombatSystem/Blueprints/BP_PlayerCharacter` OtherActor))
  (set `self.BP Player Character` _asbp_player_character)
  (if (`/Game/FlexibleCombatSystem/Blueprints/AI/BP_EnemyAI.Dead?` (`self.Enemy`))
    (bind _asbp_game_modee (cast `/Game/FlexibleCombatSystem/Blueprints/BP_GameModee` (`GameplayStatics.GetGameMode`)))
    (`/Game/FlexibleCombatSystem/Blueprints/BP_GameModee.ChangeLevelSaves` _asbp_game_modee)
    (bind _result (`BlueprintSetLibrary.Set_ToArray` _blockspeedtime))
    (for _array_element _result
      (set `self.BlockSpeedSum` (+ _array_element (`self.BlockSpeedSum`))))
    (set `self.BlockSpeedValue` (/ (`self.BlockSpeedSum`) (`BlueprintSetLibrary.Set_Length` _blockspeedtime)))
    (bind _result_2 (`BlueprintSetLibrary.Set_ToArray` _deltablock))
    (for _array_element_2 _result_2
      (set `self.DeltaBlockSum` (+ _array_element_2 (`self.DeltaBlockSum`))))
    (set `self.DeltaBlockValue` (/ (`self.DeltaBlockSum`) (`BlueprintSetLibrary.Set_Length` _deltablock)))
    (`self.SaveValues`)
    (`self.ZeroPlayerValue`)
    (if (not (`self.LastLevel`))
      (`GameplayStatics.OpenLevelBySoftObjectPtr` (`self.Level`))
      (else
        (`self.ReadValues` (`self.Arena1`))
        (`self.ReadValues` (`self.Arena2`))
        (`|ExecutionSequence`
          (:`then_0`
            (bind _value_from_file (`self.ReadFileMacros` (`KismetStringLibrary.Concat_StrStr` (`self.Arena2`) (`self.Attack LMB`)))
              (:`Ex`
                (bind _returnvalue (`KismetStringLibrary.Conv_StringToInt` _value_from_file))
                (set `self.AttackC` (- (`self.AttackC`) _returnvalue))
                (set `self.AttackInverse` _returnvalue))))
          (:`then_1`
            (bind _value_from_file_2 (`self.ReadFileMacros` (`KismetStringLibrary.Concat_StrStr` (`self.Arena2`) (`self.Blocked Counter`)))
              (:`Ex`
                (bind _returnvalue_2 (`KismetStringLibrary.Conv_StringToInt` _value_from_file_2))
                (set `self.BlockedC` (- (`self.BlockedC`) _returnvalue_2))
                (set `self.DefendInverse` _returnvalue_2))))
          (:`then_2`
            (`self.ReadValues` (`self.Arena3`))
            (`self.SetValuesToPlayer` (`self.BP Player Character`))
            (set `self.FilePath` "C:\\ResearchGame\\Final\\")
            (`self.SaveValues`)
            (`|ExecutionSequence`
              (:`then_0`
                (`self.SaveFileMacros` (`self.Block Speed Value`) (`KismetStringLibrary.Conv_DoubleToString` (`/Game/FlexibleCombatSystem/Blueprints/BP_PlayerCharacter.BlockSpeedValue` (`self.BP Player Character`)))))
              (:`then_1`
                (`self.SaveFileMacros` (`self.Delta Block Value`) (`KismetStringLibrary.Conv_DoubleToString` (`/Game/FlexibleCombatSystem/Blueprints/BP_PlayerCharacter.DeltaBlockValue` (`self.BP Player Character`)))))
              (:`then_2`
                (bind _returnvalue_3 (`|CreateWidget` "/Game/FlexibleCombatSystem/Blueprints/WB_FinalScreen.WB_FinalScreen_C" (`GameplayStatics.GetPlayerController` 0)))
                (`UserWidget.AddToViewport` _returnvalue_3 0)))))))))

(fn `ReadValues`
  (params (Arena :type String))
  (locals (ThisArena :type String))
  (set `local.ThisArena` Arena)
  (`|ExecutionSequence`
    (:`then_0`
      (bind _value_from_file (`self.ReadFileMacros` (`KismetStringLibrary.Concat_StrStr` (`local.ThisArena`) (`self.Block Speed Value`)))
        (:`Ex`
          (set `self.BlockSpeedV` (+ (`self.BlockSpeedV`) (`KismetStringLibrary.Conv_StringToDouble` _value_from_file))))))
    (:`then_1`
      (bind _value_from_file_2 (`self.ReadFileMacros` (`KismetStringLibrary.Concat_StrStr` (`local.ThisArena`) (`self.Delta Block Value`)))
        (:`Ex`
          (set `self.DeltaBlockV` (+ (`self.DeltaBlockV`) (`KismetStringLibrary.Conv_StringToDouble` _value_from_file_2))))))
    (:`then_3`
      (bind _value_from_file_3 (`self.ReadFileMacros` (`KismetStringLibrary.Concat_StrStr` (`local.ThisArena`) (`self.Player Damage Counter`)))
        (:`Ex`
          (set `self.PlayerDamageC` (+ (`self.PlayerDamageC`) (`KismetStringLibrary.Conv_StringToInt` _value_from_file_3))))))
    (:`then_4`
      (bind _value_from_file_4 (`self.ReadFileMacros` (`KismetStringLibrary.Concat_StrStr` (`local.ThisArena`) (`self.Attack LMB`)))
        (:`Ex`
          (set `self.AttackC` (+ (`self.AttackC`) (`KismetStringLibrary.Conv_StringToInt` _value_from_file_4))))))
    (:`then_5`
      (bind _value_from_file_5 (`self.ReadFileMacros` (`KismetStringLibrary.Concat_StrStr` (`local.ThisArena`) (`self.Attack Combo 2Counter`)))
        (:`Ex`
          (set `self.Combo2C` (+ (`self.Combo2C`) (`KismetStringLibrary.Conv_StringToInt` _value_from_file_5))))))
    (:`then_6`
      (bind _value_from_file_6 (`self.ReadFileMacros` (`KismetStringLibrary.Concat_StrStr` (`local.ThisArena`) (`self.Attack Combo 3Counter`)))
        (:`Ex`
          (set `self.Combo3C` (+ (`self.Combo3C`) (`KismetStringLibrary.Conv_StringToInt` _value_from_file_6))))))
    (:`then_7`
      (bind _value_from_file_7 (`self.ReadFileMacros` (`KismetStringLibrary.Concat_StrStr` (`local.ThisArena`) (`self.Attack on Block`)))
        (:`Ex`
          (set `self.AttackOnBlockC` (+ (`self.AttackOnBlockC`) (`KismetStringLibrary.Conv_StringToInt` _value_from_file_7))))))
    (:`then_8`
      (bind _value_from_file_8 (`self.ReadFileMacros` (`KismetStringLibrary.Concat_StrStr` (`local.ThisArena`) (`self.Blocked Counter`)))
        (:`Ex`
          (set `self.BlockedC` (+ (`self.BlockedC`) (`KismetStringLibrary.Conv_StringToInt` _value_from_file_8))))))
    (:`then_9`
      (bind _value_from_file_9 (`self.ReadFileMacros` (`KismetStringLibrary.Concat_StrStr` (`local.ThisArena`) (`self.Blocked Combo Counter`)))
        (:`Ex`
          (set `self.BlockedComboC` (+ (`self.BlockedComboC`) (`KismetStringLibrary.Conv_StringToInt` _value_from_file_9))))))
    (:`then_10`
      (bind _value_from_file_10 (`self.ReadFileMacros` (`KismetStringLibrary.Concat_StrStr` (`local.ThisArena`) (`self.BlockedRandomCounter`)))
        (:`Ex`
          (set `self.BlockedRandomC` (+ (`self.BlockedRandomC`) (`KismetStringLibrary.Conv_StringToInt` _value_from_file_10))))))
    (:`then_11`
      (bind _value_from_file_11 (`self.ReadFileMacros` (`KismetStringLibrary.Concat_StrStr` (`local.ThisArena`) (`self.WCounter`)))
        (:`Ex`
          (set `self.WC` (+ (`self.WC`) (`KismetStringLibrary.Conv_StringToInt` _value_from_file_11))))))
    (:`then_12`
      (bind _value_from_file_12 (`self.ReadFileMacros` (`KismetStringLibrary.Concat_StrStr` (`local.ThisArena`) (`self.SCounter`)))
        (:`Ex`
          (set `self.SC` (+ (`self.SC`) (`KismetStringLibrary.Conv_StringToInt` _value_from_file_12))))))
    (:`then_13`
      (bind _value_from_file_13 (`self.ReadFileMacros` (`KismetStringLibrary.Concat_StrStr` (`local.ThisArena`) (`self.ACounter`)))
        (:`Ex`
          (set `self.AC` (+ (`self.AC`) (`KismetStringLibrary.Conv_StringToInt` _value_from_file_13))))))
    (:`then_14`
      (bind _value_from_file_14 (`self.ReadFileMacros` (`KismetStringLibrary.Concat_StrStr` (`local.ThisArena`) (`self.DCounter`)))
        (:`Ex`
          (set `self.DC` (+ (`self.DC`) (`KismetStringLibrary.Conv_StringToInt` _value_from_file_14))))))))

(fn `SaveValues`
  (`|ExecutionSequence`
    (:`then_0`
      (`self.SaveFileMacros` (`self.Block Speed Value`) (`KismetStringLibrary.Conv_DoubleToString` (`self.BlockSpeedValue`))))
    (:`then_1`
      (`self.SaveFileMacros` (`self.Delta Block Value`) (`KismetStringLibrary.Conv_DoubleToString` (`self.DeltaBlockValue`))))
    (:`then_2`
      (`self.SaveFileMacros` (`self.Player Damage Counter`) (`KismetStringLibrary.Conv_IntToString` (`/Game/FlexibleCombatSystem/Blueprints/BP_PlayerCharacter.PlayerDamageCounter` (`self.BP Player Character`)))))
    (:`then_3`
      (`self.SaveFileMacros` (`self.Attack LMB`) (`KismetStringLibrary.Conv_IntToString` (`/Game/FlexibleCombatSystem/Blueprints/BP_PlayerCharacter.AttackLMB ` (`self.BP Player Character`)))))
    (:`then_4`
      (`self.SaveFileMacros` (`self.Attack Combo 2Counter`) (`KismetStringLibrary.Conv_IntToString` (`/Game/FlexibleCombatSystem/Blueprints/BP_PlayerCharacter.AttackCombo2Counter ` (`self.BP Player Character`)))))
    (:`then_5`
      (`self.SaveFileMacros` (`self.Attack Combo 3Counter`) (`KismetStringLibrary.Conv_IntToString` (`/Game/FlexibleCombatSystem/Blueprints/BP_PlayerCharacter.AttackCombo3Counter ` (`self.BP Player Character`)))))
    (:`then_6`
      (`self.SaveFileMacros` (`self.Attack on Block`) (`KismetStringLibrary.Conv_IntToString` (`/Game/FlexibleCombatSystem/Blueprints/BP_PlayerCharacter.AttackOnBlock ` (`self.BP Player Character`)))))
    (:`then_7`
      (`self.SaveFileMacros` (`self.Blocked Counter`) (`KismetStringLibrary.Conv_IntToString` (`/Game/FlexibleCombatSystem/Blueprints/BP_PlayerCharacter.BlockedCounter  ` (`self.BP Player Character`)))))
    (:`then_8`
      (`self.SaveFileMacros` (`self.Blocked Combo Counter`) (`KismetStringLibrary.Conv_IntToString` (`/Game/FlexibleCombatSystem/Blueprints/BP_PlayerCharacter.BlockedComboCounter ` (`self.BP Player Character`)))))
    (:`then_9`
      (`self.SaveFileMacros` (`self.BlockedRandomCounter`) (`KismetStringLibrary.Conv_IntToString` (`/Game/FlexibleCombatSystem/Blueprints/BP_PlayerCharacter.BlockedRandomCounter ` (`self.BP Player Character`)))))
    (:`then_10`
      (`self.SaveFileMacros` (`self.WCounter`) (`KismetStringLibrary.Conv_IntToString` (`/Game/FlexibleCombatSystem/Blueprints/BP_PlayerCharacter.WCounter` (`self.BP Player Character`)))))
    (:`then_11`
      (`self.SaveFileMacros` (`self.SCounter`) (`KismetStringLibrary.Conv_IntToString` (`/Game/FlexibleCombatSystem/Blueprints/BP_PlayerCharacter.SCounter` (`self.BP Player Character`)))))
    (:`then_12`
      (`self.SaveFileMacros` (`self.ACounter`) (`KismetStringLibrary.Conv_IntToString` (`/Game/FlexibleCombatSystem/Blueprints/BP_PlayerCharacter.ACounter` (`self.BP Player Character`)))))
    (:`then_13`
      (`self.SaveFileMacros` (`self.DCounter`) (`KismetStringLibrary.Conv_IntToString` (`/Game/FlexibleCombatSystem/Blueprints/BP_PlayerCharacter.DCounter` (`self.BP Player Character`)))))
    (:`then_14`
      (`self.SaveFileMacros` (`self.Attack Inverse`) (`KismetStringLibrary.Conv_IntToString` (`/Game/FlexibleCombatSystem/Blueprints/BP_PlayerCharacter.AttackInverse` (`self.BP Player Character`)))))
    (:`then_15`
      (`self.SaveFileMacros` (`self.Defend Inverse`) (`KismetStringLibrary.Conv_IntToString` (`/Game/FlexibleCombatSystem/Blueprints/BP_PlayerCharacter.DefendInverse` (`self.BP Player Character`)))))))

(fn `SetValuesToPlayer`
  (params (Player :type "/Game/FlexibleCombatSystem/Blueprints/BP_PlayerCharacter Object Reference"))
  (locals (BP_Player :type "/Game/FlexibleCombatSystem/Blueprints/BP_PlayerCharacter Object Reference") (PathDead :type String))
  (bind _output_get (set `local.BP_Player` Player))
  (set `local.PathDead` (`/Game/FlexibleCombatSystem/Blueprints/BP_PlayerCharacter.PathDeadPlayer` _output_get))
  (`|ExecutionSequence`
    (:`then_0`
      (bind _returnvalue (`self.FromDeadPlayer` (`self.Block Speed Value`)))
      (set `/Game/FlexibleCombatSystem/Blueprints/BP_PlayerCharacter.BlockSpeedValue` (+ (`KismetStringLibrary.Conv_StringToDouble` _returnvalue) (`self.BlockSpeedV`)) (`local.BP_Player`)))
    (:`then_1`
      (bind _returnvalue_2 (`self.FromDeadPlayer` (`self.Delta Block Value`)))
      (set `/Game/FlexibleCombatSystem/Blueprints/BP_PlayerCharacter.DeltaBlockValue` (+ (`KismetStringLibrary.Conv_StringToDouble` _returnvalue_2) (`self.DeltaBlockV`)) (`local.BP_Player`)))
    (:`then_3`
      (bind _returnvalue_3 (`self.FromDeadPlayer` (`self.Player Damage Counter`)))
      (set `/Game/FlexibleCombatSystem/Blueprints/BP_PlayerCharacter.PlayerDamageCounter` (+ (`KismetStringLibrary.Conv_StringToInt` _returnvalue_3) (`self.PlayerDamageC`)) (`local.BP_Player`)))
    (:`then_4`
      (bind _returnvalue_4 (`self.FromDeadPlayer` (`self.Attack LMB`)))
      (set `/Game/FlexibleCombatSystem/Blueprints/BP_PlayerCharacter.AttackLMB ` (+ (`KismetStringLibrary.Conv_StringToInt` _returnvalue_4) (`self.AttackC`)) (`local.BP_Player`)))
    (:`then_5`
      (bind _returnvalue_5 (`self.FromDeadPlayer` (`self.Attack Combo 2Counter`)))
      (set `/Game/FlexibleCombatSystem/Blueprints/BP_PlayerCharacter.AttackCombo2Counter ` (+ (`KismetStringLibrary.Conv_StringToInt` _returnvalue_5) (`self.Combo2C`)) (`local.BP_Player`)))
    (:`then_6`
      (bind _returnvalue_6 (`self.FromDeadPlayer` (`self.Attack Combo 3Counter`)))
      (set `/Game/FlexibleCombatSystem/Blueprints/BP_PlayerCharacter.AttackCombo3Counter ` (+ (`KismetStringLibrary.Conv_StringToInt` _returnvalue_6) (`self.Combo3C`)) (`local.BP_Player`)))
    (:`then_7`
      (bind _returnvalue_7 (`self.FromDeadPlayer` (`self.Attack on Block`)))
      (set `/Game/FlexibleCombatSystem/Blueprints/BP_PlayerCharacter.AttackOnBlock ` (+ (`KismetStringLibrary.Conv_StringToInt` _returnvalue_7) (`self.AttackOnBlockC`)) (`local.BP_Player`)))
    (:`then_8`
      (bind _returnvalue_8 (`self.FromDeadPlayer` (`self.Blocked Counter`)))
      (set `/Game/FlexibleCombatSystem/Blueprints/BP_PlayerCharacter.BlockedCounter  ` (+ (`KismetStringLibrary.Conv_StringToInt` _returnvalue_8) (`self.BlockedC`)) (`local.BP_Player`)))
    (:`then_9`
      (bind _returnvalue_9 (`self.FromDeadPlayer` (`self.Blocked Combo Counter`)))
      (set `/Game/FlexibleCombatSystem/Blueprints/BP_PlayerCharacter.BlockedComboCounter ` (+ (`KismetStringLibrary.Conv_StringToInt` _returnvalue_9) (`self.BlockedComboC`)) (`local.BP_Player`)))
    (:`then_10`
      (bind _returnvalue_10 (`self.FromDeadPlayer` (`self.BlockedRandomCounter`)))
      (set `/Game/FlexibleCombatSystem/Blueprints/BP_PlayerCharacter.BlockedRandomCounter ` (+ (`KismetStringLibrary.Conv_StringToInt` _returnvalue_10) (`self.BlockedRandomC`)) (`local.BP_Player`)))
    (:`then_11`
      (bind _returnvalue_11 (`self.FromDeadPlayer` (`self.WCounter`)))
      (set `/Game/FlexibleCombatSystem/Blueprints/BP_PlayerCharacter.WCounter` (+ (`KismetStringLibrary.Conv_StringToInt` _returnvalue_11) (`self.WC`)) (`local.BP_Player`)))
    (:`then_12`
      (bind _returnvalue_12 (`self.FromDeadPlayer` (`self.SCounter`)))
      (set `/Game/FlexibleCombatSystem/Blueprints/BP_PlayerCharacter.SCounter` (+ (`KismetStringLibrary.Conv_StringToInt` _returnvalue_12) (`self.SC`)) (`local.BP_Player`)))
    (:`then_13`
      (bind _returnvalue_13 (`self.FromDeadPlayer` (`self.ACounter`)))
      (set `/Game/FlexibleCombatSystem/Blueprints/BP_PlayerCharacter.ACounter` (+ (`KismetStringLibrary.Conv_StringToInt` _returnvalue_13) (`self.AC`)) (`local.BP_Player`)))
    (:`then_14`
      (bind _returnvalue_14 (`self.FromDeadPlayer` (`self.DCounter`)))
      (set `/Game/FlexibleCombatSystem/Blueprints/BP_PlayerCharacter.DCounter` (+ (`KismetStringLibrary.Conv_StringToInt` _returnvalue_14) (`self.DC`)) (`local.BP_Player`)))
    (:`then_15`
      (bind _returnvalue_15 (`self.FromDeadPlayer` (`self.Attack Inverse`)))
      (set `/Game/FlexibleCombatSystem/Blueprints/BP_PlayerCharacter.AttackInverse` (+ (`KismetStringLibrary.Conv_StringToInt` _returnvalue_15) (`self.AttackInverse`)) (`local.BP_Player`)))
    (:`then_16`
      (bind _returnvalue_16 (`self.FromDeadPlayer` (`self.Defend Inverse`)))
      (set `/Game/FlexibleCombatSystem/Blueprints/BP_PlayerCharacter.DefendInverse` (+ (`KismetStringLibrary.Conv_StringToInt` _returnvalue_16) (`self.DefendInverse`)) (`local.BP_Player`)))))

(fn `UserConstructionScript`)

(fn `ZeroPlayerValue`
  (`|ExecutionSequence`
    (:`then_0`
      (set `self.BlockSpeedV` 0.0))
    (:`then_1`
      (set `self.DeltaBlockV` 0.0))
    (:`then_2`
      (set `self.PlayerDeadC` 0))
    (:`then_3`
      (set `self.PlayerDamageC` 0))
    (:`then_4`
      (set `self.AttackC` 0))
    (:`then_5`
      (set `self.Combo2C` 0))
    (:`then_6`
      (set `self.Combo3C` 0))
    (:`then_7`
      (set `self.AttackOnBlockC` 0))
    (:`then_8`
      (set `self.BlockedC` 0))
    (:`then_9`
      (set `self.BlockedComboC` 0))
    (:`then_10`
      (set `self.BlockedRandomC` 0))
    (:`then_11`
      (set `self.WC` 0))
    (:`then_12`
      (set `self.SC` 0))
    (:`then_13`
      (set `self.AC` 0))
    (:`then_14`
      (set `self.DC` 0))
    (:`then_15`
      (set `self.AttackInverse` 0))
    (:`then_16`
      (set `self.DefendInverse` 0))))